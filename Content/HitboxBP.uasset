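; Hitbox actor that visualizes a proximity, strike or hurtbox volume, as used in fighting-style combat.
; Its SpawnHitbox event picks a material for HitboxDisplay from HitboxType, moves the display to HitboxLocation in world space without sweeping, and makes it visible.
; BeginPlay, Tick, overlap and construction logic are empty, so the Blueprint itself performs no hit detection response.
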(event Custom|SpawnHitbox
  (switch Utilities|FlowControl|Switch|SwitchonEHitboxEnum (Variables|Default|GethitboxType)
    (:HB_PROXIMITY
      (Rendering|Material|SetMaterial (Variables|Default|GetHitboxDisplay) 0 "/Game/Materials/proxHitbox.proxHitbox"))
    (:HB_STRIKE
      (Rendering|Material|SetMaterial (Variables|Default|GetHitboxDisplay) 0 "/Game/Materials/strikeHitbox.strikeHitbox"))
    (:HB_HURTBOX
      (Rendering|Material|SetMaterial (Variables|Default|GetHitboxDisplay) 0 "/Game/Materials/hurtHitbox.hurtHitbox")))
  (Transformation|SetWorldLocation (Variables|Default|GetHitboxDisplay) (Variables|Default|GethitboxLocation) false false)
  (Rendering|SetVisibility (Variables|Default|GetHitboxDisplay) true false))

(event EventBeginPlay)

(event Collision|EventActorBeginOverlap
  (params (OtherActor :type Actor%20Object%20Reference)))

(event EventTick
  (params (DeltaSeconds :type Float%20%28single-precision%29)))

(fn ConstructionScript)